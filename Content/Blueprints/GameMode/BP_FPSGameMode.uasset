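; FPS game mode for a timed "Clear the Zone" round where the player must destroy every drone before time runs out.
; A SessionState switch on Tick runs a warmup countdown with input disabled, then the game timer.
; DroneDied, PlayerDied and timer expiry lead to win, death or out-of-time states that disable input.
; It creates the HUD widget and updates its timer, drone count and announcements.
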(event `self.ReceiveBeginPlay`
  (`|ExecutionSequence`
    (:`then_0`
      ;[1 1 1] Add GameMode HUD
      (bind _returnvalue (`|CreateWidget` "/Game/Blueprints/HUD/BPW_GameModeHUD.BPW_GameModeHUD_C"))
      (bind _output_get (set `self.GameModeHUD` _returnvalue))
      (`UserWidget.AddToViewport` _output_get 0)
      (`TextBlock.SetText` (`/Game/Blueprints/HUD/BPW_GameModeHUD.AnnouncementText` _output_get) "Clear the Zone!")
      (`self.UpdateGameTimeHUD`))
    (:`then_1`
      ;[1 1 1] Set Drone Count
      (bind _outactors (`GameplayStatics.GetAllActorsOfClass` "/Game/Blueprints/Drone/BP_DronePawn.BP_DronePawn_C"))
      (set `self.NumberOfDrones` (`KismetArrayLibrary.Array_Length` _outactors))
      (`self.UpdateDroneCountHUD`))
    (:`then_2`
      (`self.DisablePlayerInput`))))

(event `self.ReceiveTick`
  (params (DeltaSeconds :type "Float (single-precision)"))
  (switch `/Game/Blueprints/GameMode/E_SessionState` (`self.SessionState`)
    (:`NewEnumerator0`
      (`self.UpdateWarmupTimer`))
    (:`NewEnumerator1`
      (`self.UpdateGameTimer` DeltaSeconds))))

(fn `DisablePlayerInput`
  (bind _returnvalue (`GameplayStatics.GetPlayerPawn` 0))
  (bind _asbp_fps_character (cast `/Game/Blueprints/Character/BP_FPS_Character` _returnvalue))
  (set `/Game/Blueprints/Character/BP_FPS_Character.bFireButtonPressed` false _asbp_fps_character)
  (`self.DisableInput` _returnvalue null))

(fn `DroneDied`
  (bind _result (`/Engine/EditorBlueprintResources/StandardMacros.DecrementInt` (`self.NumberOfDrones`))
    (:`  `
      (`self.UpdateDroneCountHUD`)
      (if (<= _result 0)
        (`self.PlayerWon`)))))

(fn `OutOfTime`
  (set `self.SessionState` "NewEnumerator2")
  (set `self.TimeRemaining` 0.0)
  (`self.UpdateGameTimeHUD`)
  (`TextBlock.SetText` (`/Game/Blueprints/HUD/BPW_GameModeHUD.AnnouncementText` (`self.GameModeHUD`)) "Out of Time!")
  (`self.DisablePlayerInput`))

(fn `PlayerDied`
  (set `self.SessionState` "NewEnumerator3")
  (`TextBlock.SetText` (`/Game/Blueprints/HUD/BPW_GameModeHUD.AnnouncementText` (`self.GameModeHUD`)) "You Died!")
  (set `self.TimeRemaining` 0.0)
  (`self.UpdateGameTimeHUD`)
  (`self.DisablePlayerInput`))

(fn `PlayerWon`
  (bind _asbp_fps_character (cast `/Game/Blueprints/Character/BP_FPS_Character` (`GameplayStatics.GetPlayerPawn` 0)))
  (if (> (`/Game/Blueprints/Character/BP_FPS_Character.Health` _asbp_fps_character) 0.0)
    (set `self.SessionState` "NewEnumerator4")
    (`TextBlock.SetText` (`/Game/Blueprints/HUD/BPW_GameModeHUD.AnnouncementText` (`self.GameModeHUD`)) "You Win!")
    (`self.DisablePlayerInput`)))

(fn `StartGame`
  (bind _returnvalue (`GameplayStatics.GetPlayerPawn` 0))
  (set `self.SessionState` "NewEnumerator1")
  (cast `PlayerController` (`Pawn.GetController` _returnvalue))
  (`self.EnableInput` _returnvalue null)
  (`TextBlock.SetText` (`/Game/Blueprints/HUD/BPW_GameModeHUD.WarmupText` (`self.GameModeHUD`)) "")
  (`TextBlock.SetText` (`/Game/Blueprints/HUD/BPW_GameModeHUD.AnnouncementText` (`self.GameModeHUD`)) ""))

(fn `TimeRemainingFormat`
  (returns (FormatTime :type Text))
  (bind _timeremaining (`self.TimeRemaining`))
  (return (`|FormatText` "{Minutes}:{Seconds}" (`KismetTextLibrary.Conv_DoubleToText` (/ _timeremaining 60.0) "ToNegativeInfinity" false true 2 2 0 0) (`KismetTextLibrary.Conv_DoubleToText` (mod _timeremaining 60.0) "ToNegativeInfinity" false true 2 2 0 0))))

(fn `UpdateDroneCountHUD`
  (`TextBlock.SetText` (`/Game/Blueprints/HUD/BPW_GameModeHUD.DronesText` (`self.GameModeHUD`)) (`KismetTextLibrary.Conv_IntToText` (`self.NumberOfDrones`))))

(fn `UpdateGameTimeHUD`
  (`TextBlock.SetText` (`/Game/Blueprints/HUD/BPW_GameModeHUD.TimeText` (`self.GameModeHUD`)) (`self.TimeRemainingFormat`))
  (if (<= (`self.TimeRemaining`) 10.0)
    (`TextBlock.SetColorAndOpacity` (`/Game/Blueprints/HUD/BPW_GameModeHUD.TimeText` (`self.GameModeHUD`)) (make `SlateColor` (struct :`R` 1.0 :`A` 1.0)))))

(fn `UpdateGameTimer`
  (params (DeltaTime :type "Float (double-precision)"))
  (bind _output_get (set `self.TimeRemaining` (- (`self.TimeRemaining`) DeltaTime)))
  (`self.UpdateGameTimeHUD`)
  (if (<= _output_get 0.0)
    (`self.OutOfTime`)))

(fn `UpdateWarmupTimer`
  (bind _returnvalue (`KismetMathLibrary.FCeil64` (- (`self.WarmupTime`) (`KismetSystemLibrary.GetGameTimeInSeconds`))))
  (`TextBlock.SetText` (`/Game/Blueprints/HUD/BPW_GameModeHUD.WarmupText` (`self.GameModeHUD`)) (`KismetTextLibrary.Conv_Int64ToText` _returnvalue))
  (if (<= _returnvalue 0)
    (`self.StartGame`)))

(fn `UserConstructionScript`)
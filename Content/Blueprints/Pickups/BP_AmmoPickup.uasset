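; Ammo pickup actor that grants ammo to the player character when touched.
; Each tick it spins its static mesh around the yaw axis at a configurable rotation rate scaled by delta time.
; When a BP_FPS_Character overlaps the pickup sphere, it adds the ammo amount, plays a 2D equip sound and destroys itself.
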(event `self.ReceiveTick`
  (params (DeltaSeconds :type "Float (single-precision)"))
  (`SceneComponent.K2_AddWorldRotation` (`self.StaticMesh`) (`KismetMathLibrary.MakeRotator` 0.0 0.0 (* DeltaSeconds (`self.RotationRate`))) false false))

(event `self.PickupSphere.OnComponentBeginOverlap`
  (params (OverlappedComponent :type "PrimitiveComponent Object Reference") (OtherActor :type "Actor Object Reference") (OtherComp :type "PrimitiveComponent Object Reference") (OtherBodyIndex :type Integer) (bFromSweep :type Boolean) (SweepResult :type "HitResult Structure (by ref)"))
  (bind _asbp_fps_character (cast `/Game/Blueprints/Character/BP_FPS_Character` OtherActor))
  (`/Game/Blueprints/Character/BP_FPS_Character.AddAmmo` _asbp_fps_character (`self.Ammo`))
  (`GameplayStatics.PlaySound2D` "/Game/Assets/Sounds/Ammo/sw_AmmoEquip.sw_AmmoEquip" 1.0 1.0 0.0 null null)
  (`self.K2_DestroyActor`))

(fn `UserConstructionScript`)